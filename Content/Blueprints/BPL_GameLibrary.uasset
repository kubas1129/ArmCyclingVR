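; BPL_GameLibrary is a Blueprint function library of shared helpers for the power network, graphics settings and object creation.
; UpdatePowerDevices recomputes power by resetting every BPI_PowerInterface actor, then telling each BP_PowerSource to update its destinations.
; LoadSettings applies a hardcoded graphics preset through console commands on player 0's controller.
; ConstructComponent wraps constructing an object from a given class and outer.
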(fn UpdatePowerDevices
  (bind ___worldcontext (LocalVariables|Get__WorldContext))
  (bind _outactors (Actor|GetAllActorswithInterface ___worldcontext "/Game/Data/Interfaces/BPI_PowerInterface.BPI_PowerInterface_C"))
  (for _array_element _outactors
    (Class|BPIPowerInterface|ResetDevice(Message) _array_element) ; Reset each power device
  )
  (bind _outactors_2 (Actor|GetAllActorsOfClass ___worldcontext "/Game/Blueprints/Mechanism/PowerUtility/BP_PowerSource.BP_PowerSource_C"))
  (for _array_element_2 _outactors_2
    (Class|BPIPowerInterface|UpdatePowerDestination(Message) _array_element_2 true))
  (return true))

(fn LoadSettings
  (bind ___worldcontext (LocalVariables|Get__WorldContext))
  (bind ___worldcontext_2 (LocalVariables|Get__WorldContext))
  (bind _returnvalue (Game|GetPlayerController ___worldcontext))
  (Development|ExecuteConsoleCommand ___worldcontext_2 "r.ScreenPercentage 60" _returnvalue)
  (Development|ExecuteConsoleCommand ___worldcontext_2 "r.ViewDistanceScale 0.7" _returnvalue)
  (Development|ExecuteConsoleCommand ___worldcontext_2 "r.PostProcessAAQuality 2" _returnvalue)
  (Development|ExecuteConsoleCommand ___worldcontext_2 "sg.PostProcessQuality 1" _returnvalue)
  (Development|ExecuteConsoleCommand ___worldcontext_2 "sg.ShadowQuality 3" _returnvalue)
  (Development|ExecuteConsoleCommand ___worldcontext_2 "sg.TextureQuality 2" _returnvalue)
  (Development|ExecuteConsoleCommand ___worldcontext_2 "sg.EffectsQuality 2" _returnvalue)
  (Development|ExecuteConsoleCommand ___worldcontext_2 "FoliageQuality 2" _returnvalue))

(fn ConstructComponent
  (params (Class :type Object%20Class%20Reference) (Outer :type Object%20Object%20Reference))
  (bind _returnvalue (Game|ConstructObjectfromClass Class Outer))
  (return _returnvalue))