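; Sliding door Blueprint that moves its static mesh along local X between closed and open positions.
; OnDoorOpen sets the open target and starts a one-shot timer of the given duration; OnDoorClose invalidates the handle and resets the target.
; Tick eases the mesh toward the target with FInterpTo.
; GetElapsedTime reports timer progress as a fraction of that duration, or -1 without a valid timer.
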(event EventTick
  (params (DeltaSeconds :type Float%20%28single-precision%29))
  (bind _staticmesh (Variables|Default|GetStaticMesh))
  (bind _relativelocation (Variables|/Script/Engine.SceneComponent|GetRelativeLocation _staticmesh))
  ;[1 1 1] Door anim
  (Transformation|SetRelativeLocation (Variables|Default|GetStaticMesh) (Math|Vector|MakeVector (Math|Interpolation|FInterpTo (.x _relativelocation) (Variables|Default|GettargetLocation) DeltaSeconds 2.0) (.y _relativelocation) (.z _relativelocation)) false false))

(event EventOnDoorOpen
  (params (time :type Float%20%28single-precision%29))
  ;[1 1 1] Open door
  (if (Utilities|Time|IsValidTimerHandle (Variables|Default|GettimerHandle))
    _
    (else
      _))
  (bind _output_get (Variables|Default|Settime time))
  (bind _returnvalue (Utilities|Time|SetTimerbyEvent (EventDispatchers|CreateEvent :!event OnDoorClose) _output_get))
  (Variables|Default|SettimerHandle _returnvalue)
  (Variables|Default|SettargetLocation 1e+02))

(event EventOnDoorClose
  ;[1 1 1] Close door
  (Utilities|Time|InvalidateTimerHandle (Variables|Default|GettimerHandle))
  (Variables|Default|SettargetLocation 0.0))

(fn ConstructionScript)

(fn GetElapsedTime
  (bind _timerhandle (Variables|Default|GettimerHandle))
  (return (select (Utilities|Time|IsValidTimerHandle _timerhandle) (/ (Class|KismetSystemLibrary|GetTimerElapsedTimeHandle _timerhandle) (Variables|Default|Gettime)) -1.0)))