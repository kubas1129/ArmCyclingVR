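; BP_Door is a power-driven door mechanism that opens while connected to a power source and closes when disconnected.
; Power updates set the connection flag and re-evaluate the door state, while a device reset clears the flag and re-evaluates after a short delay.
; An IsOpen guard gates a timeline that lerps the mesh's Z location to open and reverses to close.
; The construction script applies a configurable mesh.
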(event Custom|OpenDoor
  ;[1 1 1] Door mechanism
  (if (and (Variables|Default|GetconnectedToSource) (not (Variables|Default|GetisOpen)))
    (Variables|Default|SetisOpen true)
    (bind _alpha (Timeline|DoorTimeline Play)
      (:Update
        (Transformation|SetRelativeLocation (Variables|Default|GetStaticMesh) (Math|Vector|MakeVector 0.0 0.0 (Math|Float|Lerp 0.0 2.9e+02 _alpha)) false false)))))

(event Custom|CloseDoor
  ;[1 1 1] Door mechanism
  (if (and (not (Variables|Default|GetconnectedToSource)) (Variables|Default|GetisOpen))
    (Variables|Default|SetisOpen false)
    (bind _alpha (Timeline|DoorTimeline Reverse)
      (:Update
        (Transformation|SetRelativeLocation (Variables|Default|GetStaticMesh) (Math|Vector|MakeVector 0.0 0.0 (Math|Float|Lerp 0.0 2.9e+02 _alpha)) false false)))))

(event EventUpdatePowerDestination
  (params (powerState :type Boolean))
  ;[1 1 1] Update Power destination
  (Variables|Default|SetconnectedToSource powerState)
  (CallFunction|UpdateDoorState))

(event EventResetDevice
  ;[1 1 1] Reset device
  (Variables|Default|SetconnectedToSource false)
  (Utilities|FlowControl|Delay 0.5)
  (CallFunction|UpdateDoorState))

(fn ConstructionScript
  (Components|StaticMesh|SetStaticMesh (Variables|Default|GetStaticMesh) (Variables|Setup|Getmesh)))

(fn UpdateDoorState
  (if (Variables|Default|GetconnectedToSource)
    (CallFunction|OpenDoor)
    (else
      (CallFunction|CloseDoor))))