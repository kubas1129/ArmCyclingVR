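; Power cable mechanism piece, in an L or S version, that relays a power state to the next device and shows it through its material.
; An incoming power update swaps the material, then passes the state to the assigned receiver or, without one, to an actor found by a short sphere trace from the active receiver point.
; The construction script picks the mesh variant and starts it unpowered, and a reset event switches it off.
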(event Custom|UpdateReceiver
  (bind _powerreceiver (Variables|Setup|GetpowerReceiver))
  (bind _l_receiver (Variables|Default|GetL_Receiver))
  (bind _islversion (Variables|Setup|GetisLVersion))
  (bind _s_receiver (Variables|Default|GetS_Receiver))
  (bind _returnvalue (select _islversion _l_receiver _s_receiver))
  (bind _returnvalue_2 (Transformation|GetWorldLocation _returnvalue))
  ;[1 1 1] Check source
  (Utilities|IsValid _powerreceiver
    (:Is%20Valid
      (Class|BPIPowerInterface|UpdatePowerDestination(Message) _powerreceiver (Variables|Default|GetisPowerActive)))
    (:Is%20Not%20Valid
      (bind (_outhit _returnvalue_3) (Collision|SphereTraceForObjects _returnvalue_2 (+ _returnvalue_2 (* (Math|Vector|GetForwardVector _returnvalue) 5.0)) 8.0 (Utilities|Array|MakeArray "ObjectTypeQuery9") false (Utilities|Array|MakeArray self) "None"))
      (if _returnvalue_3
        (Class|BPIPowerInterface|UpdatePowerDestination(Message) (.HitActor (Collision|BreakHitResult _outhit)) (Variables|Default|GetisPowerActive))))))

(event EventResetDevice
  ;[1 1 1] Reset device
  (CallFunction|SetPowerActive false)
  (Variables|Default|SetisUpdated false))

(event EventUpdatePowerDestination
  (params (powerState :type Boolean))
  ;[1 1 1] Update from power destination
  (CallFunction|SetPowerActive powerState)
  (CallFunction|UpdateReceiver))

(fn ConstructionScript
  (bind _mesh (Variables|Default|Getmesh))
  (CallFunction|SetPowerActive false)
  (Components|StaticMesh|SetStaticMesh _mesh (select (Variables|Setup|GetisLVersion) "/Game/Meshes/SM_Cable_2.SM_Cable_2" "/Game/Meshes/SM_Cable_1.SM_Cable_1"))
  (Transformation|SetRelativeLocation _mesh (select (Variables|Setup|GetisLVersion) "25.000000, 0, 0" "0, 0, 0") false false))

(fn SetPowerActive
  (params (isPowerActive :type Boolean))
  (bind _output_get (Variables|Default|SetisPowerActive isPowerActive))
  (Rendering|Material|SetMaterial (Variables|Default|Getmesh) 0 (select _output_get "/Game/Materials/Cable/MI_PowerActive.MI_PowerActive" "/Game/Materials/Cable/MI_PowerInactive.MI_PowerInactive")))