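; Energy panel mechanism actor that accepts a BP_PanelScreen_4X brought into its trigger sphere.
; On overlap it remotely releases and destroys the incoming screen, then spawns a fresh copy in place through the ChildActor4 component.
; The replacement has physics simulation off and is flagged as attached to the panel.
; The sphere's collision is then disabled, so the slot fills only once.
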(event OnComponentBeginOverlap(Sphere)
  (params (OverlappedComponent :type Primitive%20Component%20Object%20Reference) (OtherActor :type Actor%20Object%20Reference) (OtherComp :type Primitive%20Component%20Object%20Reference) (OtherBodyIndex :type Integer) (bFromSweep :type Boolean) (SweepResult :type Hit%20Result%20Structure%20%28by%20ref%29))
  (bind _childactor4 (Variables|Default|GetChildActor4))
  (bind _asbp_panel_screen_4x (Utilities|Casting|CastToBP_PanelScreen_4X OtherActor))
  (Default|ReleaseActorRemotely _asbp_panel_screen_4x)
  (Actor|DestroyActor _asbp_panel_screen_4x)
  (ChildActorComponent|SetChildActorClass _childactor4 "/Game/Blueprints/Interactable/PanelScreen4X/BP_PanelScreen_4X.BP_PanelScreen_4X_C")
  (bind _asbp_panel_screen_4x_2 (Utilities|Casting|CastToBP_PanelScreen_4X (Variables|/Script/Engine.ChildActorComponent|GetChildActor _childactor4)))
  (Physics|SetSimulatePhysics (Variables|/Game/Blueprints/Interactable/PanelScreen4X/BP_PanelScreen_4X.BP_PanelScreen_4X_C|GetSM_PanelScreen4X _asbp_panel_screen_4x_2) false)
  (Variables|/Game/Blueprints/Interactable/PanelScreen4X/BP_PanelScreen_4X.BP_PanelScreen_4X_C|SetisAttachedToPanel _asbp_panel_screen_4x_2 true)
  (Collision|SetCollisionEnabled (Variables|Default|GetSphere) "NoCollision"))

(event EventBeginPlay)

(event Collision|EventActorBeginOverlap
  (params (OtherActor :type Actor%20Object%20Reference)))

(event EventTick
  (params (DeltaSeconds :type Float%20%28single-precision%29)))

(fn ConstructionScript)