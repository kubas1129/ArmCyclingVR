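; BP_TextHelper is a helper that displays a configurable text label in the level with a gentle bobbing motion.
; The construction script applies the Text and Size variables to its TextRender component.
; Every Tick sets the component's relative Z from a sine of game time, giving a slow float one unit either side of zero.
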(event EventTick
  (params (DeltaSeconds :type Float%20%28single-precision%29))
  (Transformation|SetRelativeLocation (Variables|Default|GetTextRender) (Math|Vector|MakeVector 0.0 0.0 (Math|Trig|Sin(Degrees) (* (Utilities|Time|GetTimeSeconds) 6e+01))) false false))

(fn ConstructionScript
  (Rendering|Components|TextRender|SetText (Variables|Default|GetTextRender) (Variables|Setup|Gettext))
  (Rendering|Components|TextRender|SetWorldSize (Variables|Default|GetTextRender) (Variables|Setup|Getsize)))