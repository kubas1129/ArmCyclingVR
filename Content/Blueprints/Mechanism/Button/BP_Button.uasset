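; BP_Button is a VR push button that opens a linked door for a set time when a motion controller overlaps its mesh.
; On press it sends the door an open message, sinks the button mesh and swaps to a powered material.
; A retriggerable delay restarts on repeat presses, then closes the door and resets the button.
; On BeginPlay it creates a WB_ButtonTime widget bound to the same door.
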(event OnComponentBeginOverlap(ButtonMesh)
  (params (OverlappedComponent :type Primitive%20Component%20Object%20Reference) (OtherActor :type Actor%20Object%20Reference) (OtherComp :type Primitive%20Component%20Object%20Reference) (OtherBodyIndex :type Integer) (bFromSweep :type Boolean) (SweepResult :type Hit%20Result%20Structure%20%28by%20ref%29))
  ;[1 1 1] Button action
  (Utilities|Casting|CastToBP_MotionController OtherActor)
  (Class|BPIDoorAction|OnDoorOpen(Message) (Variables|Setup|GetdoorDestination) (Variables|Setup|GetdoorTime))
  (Transformation|SetRelativeLocation (Variables|Default|GetButtonMesh) "0,5.000000, 0" false false)
  (Rendering|Material|SetMaterial (Variables|Default|GetButtonMesh) 0 "/Game/Materials/PowerStatus/MI_PowerOn.MI_PowerOn")
  (Utilities|FlowControl|RetriggerableDelay (Variables|Setup|GetdoorTime))
  (Class|BPIDoorAction|OnDoorClose(Message) (Variables|Setup|GetdoorDestination))
  (Rendering|Material|SetMaterial (Variables|Default|GetButtonMesh) 0 "/Game/Materials/Cable/MI_PowerInactive.MI_PowerInactive")
  (Transformation|SetRelativeLocation (Variables|Default|GetButtonMesh) "0,10.000000, 0" false false))

(event EventBeginPlay
  ;[1 1 1] Set door reference
  (bind _returnvalue (UserInterface|CreateWidget "/Game/Blueprints/UI/WB_ButtonTime.WB_ButtonTime_C" (Game|GetPlayerController 0) (Variables|Setup|GetdoorDestination)))
  (UserInterface|SetWidget (Variables|Default|GetWidget) _returnvalue))

(fn ConstructionScript)