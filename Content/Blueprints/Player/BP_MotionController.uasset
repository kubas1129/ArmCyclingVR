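; VR motion controller actor for either hand, setting its tracking source, labels and timer or speed-meter widget by side.
; Trigger presses sphere-trace at the grab point to grab a pickup via PhysicsHandle, else message nearby interactables; release drops and sends release messages.
; Tick drives the handle target and outlines nearby objects, while remote events allow external grab and drop.
; Rolling location samples provide mean controller speed.
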(event Custom|GatherLocationAndVelocities
  (bind _controllerlocations (Variables|Locomotion|GetcontrollerLocations))
  (bind _controllervelocities (Variables|Locomotion|GetcontrollerVelocities))
  ;[1 1 1] Gather location
  (Utilities|Array|Insert _controllerlocations (Variables|/Script/Engine.SceneComponent|GetRelativeLocation (Variables|Default|GetMotionController)))
  (Utilities|Array|RemoveIndex _controllerlocations (Utilities|Array|LastIndex _controllerlocations))
  ;[1 1 1] Compute velocities
  (Utilities|Array|Insert _controllervelocities (Controller|GetCurrentControllerVeocity))
  (Utilities|Array|RemoveIndex _controllervelocities (Utilities|Array|LastIndex _controllervelocities)))

(event Custom|TriggerAction
  (params (isLeftHand :type Boolean) (isPressed :type Boolean))
  ;[1 1 1] Trigger Action call
  (Utilities|FlowControl|Sequence
    (:then_0
      (if isPressed ; Grab/Drop mechanism
        (bind _success (Interaction|GrabActor))
        (if (not _success)
          (Interaction|TriggerInteractable true))
        (else
          (Interaction|DropActor)
          (Interaction|TriggerInteractable false))))
    (:then_1
      (Rendering|SetVisibility (Variables|Default|GetTriggerText) (not isPressed) false))))

(event Custom|RemoteGrabActor
  (params (ActorToGrab :type BP%20Pick%20Up%20Parent%20Object%20Reference) (meshToGrab :type Static%20Mesh%20Component%20Object%20Reference))
  ;[1 1 1] Remote Grab Actor (by PickUp or by staticMeshComp)
  (Utilities|IsValid ActorToGrab
    (:Is%20Valid
      (Utilities|IsValid (Variables|Default|GetgrabbedActor)
        (:Is%20Not%20Valid
          (bind _output_get (Variables|Default|SetgrabbedActor ActorToGrab))
          (Class|PhysicsHandleComponent|GrabComponentatLocation (Variables|Default|GetPhysicsHandle) (Variables|/Game/Blueprints/Pickup/BP_PickUpParent.BP_PickUpParent_C|GetItemMesh _output_get) "None" (Transformation|GetWorldLocation (Variables|Default|GetGrabPointCenter))))))
    (:Is%20Not%20Valid
      (Physics|Components|PhysicsHandle|GrabComponentatLocationwithRotation (Variables|Default|GetPhysicsHandle) meshToGrab "None" (Transformation|GetWorldLocation (Variables|Default|GetGrabPointCenter)) (Transformation|GetWorldRotation (Variables|Default|GetMotionController))))))

(event Custom|RemoteDropActor
  ;[1 1 1] Remote Drop Actor
  (Utilities|IsValid (Variables|Default|GetgrabbedActor)
    (:Is%20Valid
      (Interaction|DropActor))
    (:Is%20Not%20Valid
      (Physics|Components|PhysicsHandle|ReleaseComponent (Variables|Default|GetPhysicsHandle)))))

(event EventBeginPlay
  (bind _controllerslocationarraysize (Variables|Locomotion|GetcontrollersLocationArraySize))
  ;[1 1 1] Begin play
  (Utilities|FlowControl|Sequence
    (:then_0
      ;;[1 1 1] Set motion setup
      (Variables|/Script/HeadMountedDisplay.MotionControllerComponent|SetMotionSource (Variables|Default|GetMotionController) (select (Variables|Default|GetisLeftHand) "Left" "Right"))
      (Rendering|Components|TextRender|SetText (Variables|Default|GetSide) (select (Variables|Default|GetisLeftHand) (Utilities|Text|MakeLiteralText "L") (Utilities|Text|MakeLiteralText "R")))
      (Rendering|Components|TextRender|SetText (Variables|Default|GetTrackpadText) (Utilities|Text|ToText(String) (select (Variables|Default|GetisLeftHand) " 
 <     > 
Rotate 
" "Move")))
      ;[1 1 1] Set Timer widget
      (bind _returnvalue (UserInterface|CreateWidget (select (Variables|Default|GetisLeftHand) "/Game/Blueprints/UI/WB_GameTimer.WB_GameTimer_C" "/Game/Blueprints/UI/WB_SpeedMeter.WB_SpeedMeter_C") (Game|GetPlayerController 0)))
      (UserInterface|SetWidget (Variables|Default|GetTimer) _returnvalue))
    (:then_1
      (Utilities|Array|Resize (Variables|Locomotion|GetcontrollerLocations) _controllerslocationarraysize)
      (Utilities|Array|Resize (Variables|Locomotion|GetcontrollerVelocities) _controllerslocationarraysize)
      ;;[1 1 1] Set timer for controller
      (Utilities|Time|SetTimerbyEvent (EventDispatchers|CreateEvent :!event Custom|GatherLocationAndVelocities) 0.05 true))))

(event EventTick
  (params (DeltaSeconds :type Float%20%28single-precision%29))
  ;[1 1 1] Tick
  (Controller|UpdatePhysicsHandle)
  (Interaction|HandleOutline))

(fn ConstructionScript)

(fn GetCurrentControllerVeocity
  (bind _controllerlocations (Variables|Locomotion|GetcontrollerLocations))
  (return (/ (Math|Vector|VectorLength (- (Utilities|Array|Get(acopy) _controllerlocations 1) (Utilities|Array|Get(acopy) _controllerlocations))) 0.05)))

(fn GetMeanControllerVelocity
  (Utilities|Array|Clear (LocalVariables|GetlocalVelocities))
  (LocalVariables|Setsum 0.0)
  (bind _output_get (LocalVariables|SetlocalVelocities (Variables|Locomotion|GetcontrollerVelocities)))
  (for _array_element _output_get
    (LocalVariables|Setsum (+ (LocalVariables|Getsum) _array_element)))
  (return (/ (LocalVariables|Getsum) (Math|Conversions|ToFloat(Integer) (Utilities|Array|Length (LocalVariables|GetlocalVelocities))))))

(fn GrabActor
  (bind _array (Utilities|Array|MakeArray "ObjectTypeQuery7"))
  (bind _array_2 (Utilities|Array|MakeArray 0))
  (bind (_success _hitactor) (Controller|GetNearestActor 6.0 _array _array_2))
  (if _success
    (bind _asbp_pick_up_parent (Utilities|Casting|CastToBP_PickUpParent _hitactor)
      (:then
        (bind _output_get (Variables|Default|SetgrabbedActor _asbp_pick_up_parent))
        (Physics|Components|PhysicsHandle|GrabComponentatLocationwithRotation (Variables|Default|GetPhysicsHandle) (Variables|/Game/Blueprints/Pickup/BP_PickUpParent.BP_PickUpParent_C|GetItemMesh _output_get) "None" (Transformation|GetWorldLocation (Variables|Default|GetGrabPointCenter)) (Transformation|GetWorldRotation (Variables|Default|GetMotionController)))
        (return true))
      (:CastFailed
        (return false)))
    (else
      (return false))))

(fn UpdatePhysicsHandle
  (bind _motioncontroller (Variables|Default|GetMotionController))
  (bind _returnvalue (Transformation|GetWorldTransform _motioncontroller))
  (Class|PhysicsHandleComponent|SetTargetLocationandRotation (Variables|Default|GetPhysicsHandle) (.location _returnvalue) (.rotation _returnvalue)))

(fn DropActor
  (Physics|Components|PhysicsHandle|ReleaseComponent (Variables|Default|GetPhysicsHandle))
  (Variables|Default|SetgrabbedActor 0)
  (return true))

(fn TriggerInteractable
  (params (isPressed :type Boolean))
  (bind _array (Utilities|Array|MakeArray "ObjectTypeQuery8"))
  (bind _array_2 (Utilities|Array|MakeArray 0))
  (bind _array_3 (Utilities|Array|MakeArray "ObjectTypeQuery8"))
  (bind _array_4 (Utilities|Array|MakeArray 0))
  (bind (_hitactor _success) (Controller|GetNearestActors 8.0 _array _array_2))
  (bind (_hitactor_2 _success_2) (Controller|GetNearestActors 8.0 _array_3 _array_4))
  (if isPressed
    (if _success
      (for _array_element _hitactor
        (if (!= (Variables|Default|GetgrabbedActor) (.HitActor (Collision|BreakHitResult _array_element)))
          (Class|BPITriggerActionInterface|OnInteractablePressed(Message) (.HitActor (Collision|BreakHitResult _array_element)) self))))
    (elif _success_2
      (for _array_element_2 _hitactor_2
        (if (!= (Variables|Default|GetgrabbedActor) (.HitActor (Collision|BreakHitResult _array_element_2)))
          (Class|BPITriggerActionInterface|OnInteractableReleased(Message) (.HitActor (Collision|BreakHitResult _array_element_2)) self))))))

(fn GetNearestActor
  (params (Radius :type Float%20%28single-precision%29) (ObjectTypes :type Array%20of%20EObjectTypeQuery%20Enums :default "ObjectTypeQuery1") (ActorsToIgnore :type Array%20of%20Actor%20Object%20References))
  (bind _grabpointcenter (Variables|Default|GetGrabPointCenter))
  (bind _returnvalue (Transformation|GetWorldLocation _grabpointcenter))
  (bind (_outhit _returnvalue_2) (Collision|SphereTraceForObjects _returnvalue (+ _returnvalue 0.1) Radius ObjectTypes false ActorsToIgnore "None"))
  (if _returnvalue_2
    (return _returnvalue_2 (.HitActor (Collision|BreakHitResult _outhit)))
    (else
      (return false 0))))

(fn HandleOutline
  (bind _array (Utilities|Array|MakeArray "ObjectTypeQuery7" "ObjectTypeQuery8"))
  (bind _array_2 (Utilities|Array|MakeArray 0))
  (bind (_success _hitactor) (Controller|GetNearestActor 6.0 _array _array_2))
  (if _success
    (Class|BPIItemInteraction|UpdateOutline(Message) _hitactor)))

(fn GetNearestActors
  (params (Radius :type Float%20%28single-precision%29) (ObjectTypes :type Array%20of%20EObjectTypeQuery%20Enums :default "ObjectTypeQuery1") (ActorsToIgnore :type Array%20of%20Actor%20Object%20References))
  (bind _grabpointcenter (Variables|Default|GetGrabPointCenter))
  (bind _returnvalue (Transformation|GetWorldLocation _grabpointcenter))
  (bind (_outhits _returnvalue_2) (Collision|MultiSphereTraceForObjects _returnvalue (+ _returnvalue 0.1) Radius ObjectTypes false ActorsToIgnore "None"))
  (return _outhits _returnvalue_2))

(fn ResetVelocities
  (bind _controllervelocities (Variables|Locomotion|GetcontrollerVelocities))
  (Utilities|Array|Clear _controllervelocities)
  (Utilities|Array|Resize _controllervelocities (Variables|Locomotion|GetcontrollersLocationArraySize)))