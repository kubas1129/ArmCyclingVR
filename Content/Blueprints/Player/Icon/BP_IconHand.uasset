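; BP_IconHand is a hand icon actor that shows a material billboard on a target component when the player's camera is nearby.
; On BeginPlay its Scene component snaps to AttachComponent's location and rotation while keeping world scale.
; Every Tick it compares the camera-to-AttachComponent distance with Radius and shows the billboard only within that range.
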(event EventBeginPlay
  (Transformation|AttachComponentToComponent (Variables|Default|GetScene) (Variables|Default|GetattachComponent) "None" "SnapToTarget" "SnapToTarget" "KeepWorld" true))

(event EventTick
  (params (DeltaSeconds :type Float%20%28single-precision%29))
  (Rendering|SetVisibility (Variables|Default|GetMaterialBillboard) (<= (Math|Vector|VectorLength (- (Transformation|GetActorLocation (Game|GetPlayerCameraManager 0)) (Transformation|GetWorldLocation (Variables|Default|GetattachComponent)))) (Variables|Default|Getradius)) false))

(fn ConstructionScript)