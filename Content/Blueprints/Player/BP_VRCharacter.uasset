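; VR player character that spawns left and right motion controllers on the VR origin with floor tracking, and adjusts origin and camera when no headset is active.
; Trackpad input moves along a pitch-free camera heading, while held controller-move input walks forward at a speed scaled by average hand velocity, shown as text.
; MovementMode keeps these two schemes mutually exclusive.
; Separate axes provide camera-relative movement and look without mode checks.
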(event EventBeginPlay
  (bind _vrorigin (Variables|Default|GetVROrigin))
  (bind _relativelocation (Variables|/Script/Engine.SceneComponent|GetRelativeLocation _vrorigin))
  ;[1 1 1] Begin Play
  (CallFunction|InitSetup)
  (if (not (Class|HeadMountedDisplayFunctionLibrary|IsHeadMountedDisplayEnabled))
    (Transformation|SetRelativeLocation _vrorigin (Math|Vector|MakeVector (.x _relativelocation) (.y _relativelocation) 9e+01) false false)
    (Variables|/Script/Engine.CameraComponent|SetbUsePawnControlRotation (Variables|Default|GetVRCamera) true)))

(event Input|AxisEvents|InputAxisMoveForward
  (params (AxisValue :type Float%20%28single-precision%29))
  ;[1 1 1] Move by keyboard
  (Pawn|Input|AddMovementInput (Math|Vector|GetForwardVector (Variables|Default|GetVRCamera)) AxisValue false))

(event Input|AxisEvents|InputAxisMoveRight
  (params (AxisValue :type Float%20%28single-precision%29))
  ;[1 1 1] Move by keyboard
  (Pawn|Input|AddMovementInput (Math|Vector|GetRightVector (Variables|Default|GetVRCamera)) AxisValue false))

(event Input|AxisEvents|InputAxisTurn
  (params (AxisValue :type Float%20%28single-precision%29))
  (Pawn|Input|AddControllerYawInput AxisValue))

(event Input|AxisEvents|InputAxisTrackPadMoveForward
  (params (AxisValue :type Float%20%28single-precision%29))
  ;[1 1 1] Movement by trackpad
  (switch Utilities|FlowControl|Switch|SwitchonE_VRMovementMode (Variables|Default|GetmovementMode)
    (:NewEnumerator2
      _)
    (:NewEnumerator0
      _))
  (Math|Float|CompareFloat AxisValue 0.0
    (:>
      (Variables|/Script/Engine.CharacterMovementComponent|SetMaxWalkSpeed (Variables|Character|GetCharacterMovement) 5e+02 :!label _label)
      (Pawn|Input|AddMovementInput (Math|Vector|GetForwardVector (CallFunction|GetFixedCameraRotation)) AxisValue false)
      (Variables|Default|SetmovementMode "NewEnumerator0"))
    (:==
      (Variables|Default|SetmovementMode "NewEnumerator2"))
    (:<
      (goto _label))))

(event Input|AxisEvents|InputAxisTrackPadMoveRight
  (params (AxisValue :type Float%20%28single-precision%29))
  ;[1 1 1] Movement by trackpad
  (switch Utilities|FlowControl|Switch|SwitchonE_VRMovementMode (Variables|Default|GetmovementMode)
    (:NewEnumerator2
      _)
    (:NewEnumerator0
      _))
  (Math|Float|CompareFloat AxisValue 0.0
    (:>
      (Variables|/Script/Engine.CharacterMovementComponent|SetMaxWalkSpeed (Variables|Character|GetCharacterMovement) 5e+02 :!label _label)
      (Pawn|Input|AddMovementInput (Math|Vector|GetRightVector (CallFunction|GetFixedCameraRotation)) AxisValue false)
      (Variables|Default|SetmovementMode "NewEnumerator0"))
    (:==
      (Variables|Default|SetmovementMode "NewEnumerator2"))
    (:<
      (goto _label))))

(event Input|AxisEvents|InputAxisActivateControllersMove
  (params (AxisValue :type Float%20%28single-precision%29))
  (bind _vrcamera (Variables|Default|GetVRCamera))
  (bind _returnvalue (Transformation|GetWorldRotation _vrcamera))
  ;[1 1 1] Move by controllers
  (switch Utilities|FlowControl|Switch|SwitchonE_VRMovementMode (Variables|Default|GetmovementMode)
    (:NewEnumerator2
      _)
    (:NewEnumerator1
      _))
  (Math|Float|CompareFloat AxisValue 0.0
    (:>
      (Utilities|FlowControl|Sequence
        (:then_0
          (bind _mean (CallFunction|ComputeHandsVelocity))
          (if (> _mean 1.0)
            (Variables|/Script/Engine.CharacterMovementComponent|SetMaxWalkSpeed (Variables|Character|GetCharacterMovement) (Math|Float|Lerp 0.0 5e+02 (/ _mean 2e+01)))
            (Pawn|Input|AddMovementInput (Math|Vector|GetForwardVector (Math|Rotator|MakeRotator (.roll _returnvalue) 0.0 (.yaw _returnvalue))) 1.0 false))
          (Rendering|Components|TextRender|SetText (Variables|Default|GetTextRender) (Utilities|Text|ToText(Float) _mean "HalfToEven"))
          (Variables|Default|SetmovementMode "NewEnumerator1"))
        (:then_1
          (goto _label Reset))))
    (:==
      (Utilities|FlowControl|DoOnce false :!label _label
        (:Completed
          (Variables|Default|SetmovementMode "NewEnumerator2"))))))

(event Input|AxisEvents|InputAxisLookUp
  (params (AxisValue :type Float%20%28single-precision%29))
  (Pawn|Input|AddControllerPitchInput AxisValue))

(fn ConstructionScript)

(fn InitSetup
  (bind _vrorigin (Variables|Default|GetVROrigin))
  (bind _relativelocation (Variables|/Script/Engine.SceneComponent|GetRelativeLocation _vrorigin))
  ;[1 1 1] Spawn and attach controllers
  (bind _returnvalue (Game|SpawnActorfromClass "/Game/Blueprints/Player/BP_MotionController.BP_MotionController_C" (Transformation|GetActorTransform) "Undefined" self false 0))
  (bind _output_get (Variables|Default|SetrightHandRef _returnvalue))
  (Transformation|AttachComponentToComponent _output_get (Variables|Default|GetVROrigin) "None" "SnapToTarget" "SnapToTarget" "KeepWorld" true)
  (bind _returnvalue_2 (Game|SpawnActorfromClass "/Game/Blueprints/Player/BP_MotionController.BP_MotionController_C" (Transformation|GetActorTransform) "Undefined" self true 0))
  (bind _output_get_2 (Variables|Default|SetleftHandRef _returnvalue_2))
  (Transformation|AttachComponentToComponent _output_get_2 (Variables|Default|GetVROrigin) "None" "SnapToTarget" "SnapToTarget" "KeepWorld" true)
  ;[1 1 1] Set origin location and proper tracking origin
  (Class|HeadMountedDisplayFunctionLibrary|SetTrackingOrigin "Floor") ; Windows (Oculus / Vive)
  (Transformation|SetRelativeLocation _vrorigin (Math|Vector|MakeVector (.x _relativelocation) (.y _relativelocation) -9e+01) false false))

(fn ComputeHandsVelocity
  (return (/ (+ (Default|GetMeanControllerVelocity (Variables|Default|GetrightHandRef)) (Default|GetMeanControllerVelocity (Variables|Default|GetleftHandRef))) 2.0)))

(fn GetFixedCameraRotation
  (bind _vrcamera (Variables|Default|GetVRCamera))
  (bind _returnvalue (Transformation|GetWorldRotation _vrcamera))
  (return (Math|Rotator|MakeRotator (.roll _returnvalue) 0.0 (.yaw _returnvalue))))