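; BP_MotionController is a VR hand controller that tracks how fast the hand moves, with its motion source set to left or right on BeginPlay.
; A looping 0.05-second timer samples the controller's relative location into fixed-size rolling histories of locations and velocities.
; Each velocity is the distance between the two newest samples, not divided by time.
; GetMeanControllerVelocity averages that history to give a smoothed speed.
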(event Custom|GatherLocationAndVelocities
  (bind _controllerlocations (Variables|Default|GetcontrollerLocations))
  (bind _controllervelocities (Variables|Default|GetcontrollerVelocities))
  ;[1 1 1] Gather location
  (Utilities|Array|Insert _controllerlocations (Variables|/Script/Engine.SceneComponent|GetRelativeLocation (Variables|Default|GetMotionController)))
  (Utilities|Array|RemoveIndex _controllerlocations (Utilities|Array|LastIndex _controllerlocations))
  ;[1 1 1] Compute velocities
  (Utilities|Array|Insert _controllervelocities (CallFunction|GetCurrentControllerVeocity))
  (Utilities|Array|RemoveIndex _controllervelocities (Utilities|Array|LastIndex _controllervelocities)))

(event EventBeginPlay
  (bind _controllerslocationarraysize (Variables|Default|GetcontrollersLocationArraySize))
  (Utilities|FlowControl|Sequence
    (:then_0
      ;[1 1 1] Set motion setup
      (Variables|/Script/HeadMountedDisplay.MotionControllerComponent|SetMotionSource (Variables|Default|GetMotionController) (select (Variables|Default|GetisLeftHand) "Left" "Right")))
    (:then_1
      (Utilities|Array|Resize (Variables|Default|GetcontrollerLocations) _controllerslocationarraysize)
      (Utilities|Array|Resize (Variables|Default|GetcontrollerVelocities) _controllerslocationarraysize)
      ;[1 1 1] Set timer for controller
      (Utilities|Time|SetTimerbyEvent (EventDispatchers|CreateEvent :!event Custom|GatherLocationAndVelocities) 0.05 true))))

(fn ConstructionScript)

(fn GetCurrentControllerVeocity
  (bind _controllerlocations (Variables|Default|GetcontrollerLocations))
  (return (Math|Vector|VectorLength (- (Utilities|Array|Get(acopy) _controllerlocations 1) (Utilities|Array|Get(acopy) _controllerlocations)))))

(fn GetMeanControllerVelocity
  (Utilities|Array|Clear (LocalVariables|GetlocalVelocities))
  (LocalVariables|Setsum 0.0)
  (bind _output_get (LocalVariables|SetlocalVelocities (Variables|Default|GetcontrollerVelocities)))
  (for _array_element _output_get
    (LocalVariables|Setsum (+ (LocalVariables|Getsum) _array_element)))
  (return (/ (LocalVariables|Getsum) (Math|Conversions|ToFloat(Integer) (Utilities|Array|Length (LocalVariables|GetlocalVelocities))))))