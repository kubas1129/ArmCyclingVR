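; BP_PickUpParent is a base Blueprint for physics-driven pickup items, with empty press and release events as action hooks.
; The construction script applies the configurable mesh, mass and first-slot material to ItemMesh.
; BeginPlay enables physics simulation and reapplies the mass override.
; UpdateOutline turns on custom depth, using a short retriggerable delay so the highlight clears itself once calls stop.
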(event EventBeginPlay
  (Physics|SetSimulatePhysics (Variables|Default|GetItemMesh) true)
  (Class|PrimitiveComponent|SetMassOverrideinKg (Variables|Default|GetItemMesh) "None" (Variables|Setup|Getmass) true))

(event Collision|EventActorBeginOverlap
  (params (OtherActor :type Actor%20Object%20Reference)))

(event EventTick
  (params (DeltaSeconds :type Float%20%28single-precision%29)))

(event EventOnPickupPressed
  (params (motionController :type BP%20Motion%20Controller%20Object%20Reference))
  ;[1 1 1] On trigger action
)

(event EventOnPickupReleased
  ;[1 1 1] On trigger action
)

(event EventUpdateOutline
  (bind _itemmesh (Variables|Default|GetItemMesh))
  ;[1 1 1] Update Outline
  (Rendering|SetRenderCustomDepth _itemmesh true)
  (Utilities|FlowControl|RetriggerableDelay 0.1)
  (Rendering|SetRenderCustomDepth _itemmesh false))

(fn ConstructionScript
  (Components|StaticMesh|SetStaticMesh (Variables|Default|GetItemMesh) (Variables|Setup|Getmesh))
  (Class|PrimitiveComponent|SetMassOverrideinKg (Variables|Default|GetItemMesh) "None" (Variables|Setup|Getmass) true)
  (Rendering|Material|SetMaterial (Variables|Default|GetItemMesh) 0 (Variables|Setup|GetmeshMaterial)))