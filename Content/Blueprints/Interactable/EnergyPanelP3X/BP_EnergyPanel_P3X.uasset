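; Three-slot energy panel that accepts BP_EnergyCube actors and powers a receiver when all slots are filled.
; Overlapping an empty holder releases and attaches the cube, then updates each slot's status material and messages PowerReceiver.
; UpdatePowerDestination checks two upstream power sources, enabling the holders when both are active.
; Losing power detaches cubes, disables collision on the holders they occupied and greys out the status indicators, without notifying the receiver.
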(event OnComponentBeginOverlap(CubeHolder_1)
  (params (OverlappedComponent :type Primitive%20Component%20Object%20Reference) (OtherActor :type Actor%20Object%20Reference) (OtherComp :type Primitive%20Component%20Object%20Reference) (OtherBodyIndex :type Integer) (bFromSweep :type Boolean) (SweepResult :type Hit%20Result%20Structure%20%28by%20ref%29))
  ;[1 1 1] Cube holder interaction
  (if (CallFunction|IsHolderEmpty (Variables|Default|GetCubeHolder_1))
    (bind _asbp_energy_cube (Utilities|Casting|CastToBP_EnergyCube OtherActor))
    (bind _success (Default|ReleaseActorRemotely _asbp_energy_cube))
    (if _success
      _
      (else
        _))
    (Default|AttachtoPanel _asbp_energy_cube (Variables|Default|GetCubeHolder_1))
    (CallFunction|UpdatePowerState)))

(event OnComponentBeginOverlap(CubeHolder_2)
  (params (OverlappedComponent :type Primitive%20Component%20Object%20Reference) (OtherActor :type Actor%20Object%20Reference) (OtherComp :type Primitive%20Component%20Object%20Reference) (OtherBodyIndex :type Integer) (bFromSweep :type Boolean) (SweepResult :type Hit%20Result%20Structure%20%28by%20ref%29))
  ;[1 1 1] Cube holder interaction
  (if (CallFunction|IsHolderEmpty (Variables|Default|GetCubeHolder_2))
    (bind _asbp_energy_cube (Utilities|Casting|CastToBP_EnergyCube OtherActor))
    (bind _success (Default|ReleaseActorRemotely _asbp_energy_cube))
    (if _success
      _
      (else
        _))
    (Default|AttachtoPanel _asbp_energy_cube (Variables|Default|GetCubeHolder_2))
    (CallFunction|UpdatePowerState)))

(event OnComponentBeginOverlap(CubeHolder_3)
  (params (OverlappedComponent :type Primitive%20Component%20Object%20Reference) (OtherActor :type Actor%20Object%20Reference) (OtherComp :type Primitive%20Component%20Object%20Reference) (OtherBodyIndex :type Integer) (bFromSweep :type Boolean) (SweepResult :type Hit%20Result%20Structure%20%28by%20ref%29))
  ;[1 1 1] Cube holder interaction
  (if (CallFunction|IsHolderEmpty (Variables|Default|GetCubeHolder_3))
    (bind _asbp_energy_cube (Utilities|Casting|CastToBP_EnergyCube OtherActor))
    (bind _success (Default|ReleaseActorRemotely _asbp_energy_cube))
    (if _success
      _
      (else
        _))
    (Default|AttachtoPanel _asbp_energy_cube (Variables|Default|GetCubeHolder_3))
    (CallFunction|UpdatePowerState)))

(event EventUpdatePowerDestination
  (params (powerState :type Boolean))
  ;[1 1 1] Update power status
  (CallFunction|CheckPowerStatus))

(fn ConstructionScript)

(fn UpdatePowerState
  (Rendering|Material|SetMaterial (Variables|Default|GetStatus_1) 0 (select (CallFunction|IsHolderEmpty (Variables|Default|GetCubeHolder_1)) "/Game/Materials/PowerStatus/MI_PowerOFf.MI_PowerOff" "/Game/Materials/PowerStatus/MI_PowerOn.MI_PowerOn"))
  (Rendering|Material|SetMaterial (Variables|Default|GetStatus_2) 0 (select (CallFunction|IsHolderEmpty (Variables|Default|GetCubeHolder_2)) "/Game/Materials/PowerStatus/MI_PowerOFf.MI_PowerOff" "/Game/Materials/PowerStatus/MI_PowerOn.MI_PowerOn"))
  (Rendering|Material|SetMaterial (Variables|Default|GetStatus_3) 0 (select (CallFunction|IsHolderEmpty (Variables|Default|GetCubeHolder_3)) "/Game/Materials/PowerStatus/MI_PowerOFf.MI_PowerOff" "/Game/Materials/PowerStatus/MI_PowerOn.MI_PowerOn"))
  (Class|BPIPowerInterface|UpdatePowerDestination(Message) (Variables|Setup|GetpowerReceiver) (Math|Boolean|ANDBoolean (not (CallFunction|IsHolderEmpty (Variables|Default|GetCubeHolder_3))) (not (CallFunction|IsHolderEmpty (Variables|Default|GetCubeHolder_2))) (not (CallFunction|IsHolderEmpty (Variables|Default|GetCubeHolder_1)))))
  (Development|PrintString "Hello"))

(fn IsHolderEmpty
  (params (comp :type Scene%20Component%20Object%20Reference))
  (return (== (Class|SceneComponent|GetNumChildrenComponents comp) 0)))

(fn CheckPowerStatus
  (bind _powersource1 (Variables|Setup|GetpowerSource1))
  (bind _powersource2 (Variables|Setup|GetpowerSource2))
  (Utilities|IsValid _powersource1
    (:Is%20Valid
      (if (Variables|/Game/Blueprints/Mechanism/PowerUtility/BP_PowerCable.BP_PowerCable_C|GetisPowerActive _powersource1)
        (Utilities|IsValid _powersource2
          (:Is%20Valid
            (if (Variables|/Game/Blueprints/Mechanism/PowerUtility/BP_PowerCable.BP_PowerCable_C|GetisPowerActive _powersource2)
              (Holder|ActivateHolder)
              (else
                (Holder|DeactivateHolder)))))
        (else
          (Holder|DeactivateHolder))))))

(fn DeactivateHolder
  (Holder|RemoteDetachfromHolder (Variables|Default|GetCubeHolder_1))
  (Holder|RemoteDetachfromHolder (Variables|Default|GetCubeHolder_2))
  (Holder|RemoteDetachfromHolder (Variables|Default|GetCubeHolder_3))
  (Rendering|Material|SetMaterial (Variables|Default|GetStatus_2) 0 "/Game/Materials/PowerStatus/MI_Inactive.MI_Inactive"))

(fn ActivateHolder
  (Collision|SetCollisionEnabled (Variables|Default|GetCubeHolder_1) "QueryAndPhysics")
  (Collision|SetCollisionEnabled (Variables|Default|GetCubeHolder_2) "QueryAndPhysics")
  (Collision|SetCollisionEnabled (Variables|Default|GetCubeHolder_3) "QueryAndPhysics")
  (Rendering|Material|SetMaterial (Variables|Default|GetStatus_2) 0 "/Game/Materials/PowerStatus/MI_PowerOFf.MI_PowerOff"))

(fn RemoteDetachfromHolder
  (params (holder :type Primitive%20Component%20Object%20Reference))
  (bind _overlappingactors (Collision|GetOverlappingActors holder "/Game/Blueprints/Interactable/EnergyPanelP3X/BP_EnergyCube.BP_EnergyCube_C" :!class /Script/Engine.PrimitiveComponent))
  (if (Utilities|Array|IsValidIndex _overlappingactors)
    (bind _asbp_energy_cube (Utilities|Casting|CastToBP_EnergyCube (Utilities|Array|Get(acopy) _overlappingactors)))
    (Default|DetachfromPanel _asbp_energy_cube)
    (Collision|SetCollisionEnabled holder "NoCollision")))