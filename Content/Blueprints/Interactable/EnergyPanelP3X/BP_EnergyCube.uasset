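; BP_EnergyCube is a grabbable energy cube that can be seated in an energy panel.
; Pressing detaches it, restores physics and has the motion controller remote-grab its mesh; releasing drops it unless it is attached.
; AttachToPanel snaps the mesh to a given component, and detaching from a BP_EnergyPanel_P3X tells that panel to update its power state.
; An outline event flashes custom depth through a short retriggerable delay.
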(event Custom|AttachToPanel
  (params (component :type Scene%20Component%20Object%20Reference))
  ;[1 1 1] Attach to panel
  (Variables|Default|SetisAttachedToPanel true)
  (Transformation|AttachComponentToComponent (Variables|Default|Getmesh) component "None" "SnapToTarget" "SnapToTarget" "KeepRelative" true))

(event EventBeginPlay
  (|CallParentFunction) ; This node is disabled and will not be called.\nDrag off pins to build functionality.
)

(event EventOnInteractablePressed
  (params (motionController :type BP%20Motion%20Controller%20Object%20Reference))
  ;[1 1 1] Interaction pressed
  (CallFunction|DetachfromPanel)
  (Default|RemoteGrabActor motionController 0 (Variables|Default|Getmesh)))

(event EventOnInteractableReleased
  (params (motionController :type BP%20Motion%20Controller%20Object%20Reference))
  ;[1 1 1] Interaction released
  (if (not (Variables|Default|GetisAttachedToPanel))
    (Default|RemoteDropActor motionController)))

(event EventUpdateOutline
  ;[1 1 1] Update outline
  (Rendering|SetRenderCustomDepth (Variables|Default|Getmesh) true)
  (Utilities|FlowControl|RetriggerableDelay 0.2)
  (Rendering|SetRenderCustomDepth (Variables|Default|Getmesh) false))

(event EventTick
  (params (DeltaSeconds :type Float%20%28single-precision%29))
  (|CallParentFunction DeltaSeconds) ; This node is disabled and will not be called.\nDrag off pins to build functionality.
)

(event Collision|EventActorBeginOverlap
  (params (OtherActor :type Actor%20Object%20Reference))
  (|CallParentFunction OtherActor) ; This node is disabled and will not be called.\nDrag off pins to build functionality.
)

(fn ConstructionScript
  (|CallParentFunction))

(fn DetachfromPanel
  (bind _mesh (Variables|Default|Getmesh))
  (if (Variables|Default|GetisAttachedToPanel)
    (Variables|Default|SetisAttachedToPanel false)
    (bind _asbp_energy_panel_p3x (Utilities|Casting|CastToBP_EnergyPanel_P3X (Components|GetOwner (Transformation|GetAttachParent _mesh)))
      (:then
        (Transformation|DetachFromComponent _mesh "KeepWorld" "KeepWorld" "KeepWorld" true)
        (Default|UpdatePowerState _asbp_energy_panel_p3x))
      (:CastFailed
        (Transformation|DetachFromComponent _mesh "KeepWorld" "KeepWorld" "KeepWorld" true)))
    (Physics|SetSimulatePhysics (Variables|Default|Getmesh) true)))