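; Interactable power-routing panel piece with an S or L conduit variant that shows active or inactive power through its material.
; When attached to a panel, releasing the interaction rotates it 90 degrees and refreshes power devices; loose pieces simulate physics and can be remote-grabbed.
; Power updates propagate through short sphere traces from two variant-specific arrows to neighboring actors, with an IsUpdated flag blocking repeat visits until reset.
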(event EventBeginPlay
  ;[1 1 1] Begin play
  (CallFunction|Init))

(event EventOnInteractablePressed
  (params (motionController :type BP%20Motion%20Controller%20Object%20Reference))
  ;[1 1 1] Interaction pressed
  (if (not (Variables|Setup|GetisAttachedToPanel))
    (Default|RemoteGrabActor motionController 0 (Variables|Default|GetSM_PanelScreen4X))))

(event EventOnInteractableReleased
  (params (motionController :type BP%20Motion%20Controller%20Object%20Reference))
  ;[1 1 1] Interaction released
  (if (Variables|Setup|GetisAttachedToPanel)
    (CallFunction|RotatePanel)
    (else
      (Default|RemoteDropActor motionController))))

(event EventUpdateOutline
  ;[1 1 1] Update outline
  (Rendering|SetRenderCustomDepth (Variables|Default|GetSM_PanelScreen4X) true)
  (Utilities|FlowControl|RetriggerableDelay 0.2)
  (Rendering|SetRenderCustomDepth (Variables|Default|GetSM_PanelScreen4X) false))

(event EventResetDevice
  ;[1 1 1] Reset device
  (CallFunction|SetActivePower false)
  (Variables|Default|SetisUpdated false))

(event EventUpdatePowerDestination
  (params (powerState :type Boolean))
  ;[1 1 1] Update power destination
  (if (not (Variables|Default|GetisUpdated))
    (CallFunction|SetActivePower powerState)
    (Variables|Default|SetisUpdated true)
    (CallFunction|UpdateConnected (select (Variables|Setup|GetLVersion) (Variables|Default|GetArrow) (Variables|Default|GetArrow1)))
    (CallFunction|UpdateConnected (select (Variables|Setup|GetLVersion) (Variables|Default|GetArrow3) (Variables|Default|GetArrow2)))))

(fn ConstructionScript
  (CallFunction|Init))

(fn RotatePanel
  (Transformation|AddRelativeRotation (Variables|Default|GetSM_PanelScreen4X) "0.000000,0.000000,-90.000000" false false)
  (CallFunction|UpdatePowerDevices))

(fn UpdateConnected
  (params (Target :type Primitive%20Component%20Object%20Reference))
  (bind _returnvalue (Transformation|GetWorldLocation Target))
  (bind (_outhit _returnvalue_2) (Collision|SphereTraceForObjects _returnvalue (+ _returnvalue (* (Math|Vector|GetForwardVector Target) 5.0)) 4.0 (Utilities|Array|MakeArray "ObjectTypeQuery2" "ObjectTypeQuery9") false (Utilities|Array|MakeArray self) "None"))
  (if _returnvalue_2
    (Class|BPIPowerInterface|UpdatePowerDestination(Message) (.HitActor (Collision|BreakHitResult _outhit)) (Variables|Default|GetpowerState))
    (return true)
    (else
      (return false))))

(fn Init
  (bind _lversion (Variables|Setup|GetLVersion))
  (bind _lmesh (Variables|Default|GetLMesh))
  (bind _smesh (Variables|Default|GetSMesh))
  (Physics|SetSimulatePhysics (Variables|Default|GetSM_PanelScreen4X) (select (Variables|Setup|GetisAttachedToPanel) false true))
  (Rendering|SetVisibility _smesh (not _lversion) true)
  (Collision|SetCollisionEnabled _smesh (select _lversion "NoCollision" "QueryAndPhysics"))
  (Rendering|SetVisibility _lmesh _lversion true)
  (Collision|SetCollisionEnabled _lmesh (select _lversion "QueryAndPhysics" "NoCollision")))

(fn SetActivePower
  (params (isPowerActive :type Boolean))
  (bind _output_get (Variables|Default|SetpowerState isPowerActive))
  (Rendering|Material|SetMaterial (Variables|Default|GetLMesh) 0 (select _output_get "/Game/Materials/Cable/MI_PowerActive.MI_PowerActive" "/Game/Materials/Cable/MI_PowerInactive.MI_PowerInactive")))